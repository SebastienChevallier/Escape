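; BP_PictureEnigme is a picture puzzle that reveals its item meshes as the player completes its tasks.
; It overrides the parent's CompleteTask, finds the completed task's index in TaskList and makes the matching one of three item meshes visible.
; The event graph holds only empty events and an unconnected, never-executed loop that would reveal the same meshes from a PicturePickup array.
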(event EventBeginPlay
  (|CallParentFunction) ; This node is disabled and will not be called.\nDrag off pins to build functionality.
)

(event Collision|EventActorBeginOverlap
  (params (OtherActor :type Actor%20Object%20Reference)))

(event EventTick
  (params (DeltaSeconds :type Float%20%28single-precision%29)))

(event EventBeginPlay)

(fn ConstructionScript
  (|CallParentFunction))

(fn CompleteTask
  (params (CurrentTask :type BP%20Task%20Object%20Reference) (Player :type BP%20First%20Person%20Character%20Object%20Reference))
  (|CallParentFunction 0 0)
  (for _index (range 0 3)
    (if (== (Utilities|Array|Get(acopy) (Variables|Default|GetTaskList) _index) CurrentTask)
      (Rendering|SetVisibility (Utilities|Array|Get(acopy) (Utilities|Array|MakeArray (Variables|Default|GetItemMesh) (Variables|Default|GetItemMesh1) (Variables|Default|GetItemMesh2)) _index) true false))))