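; BP_Enigme is a puzzle controller that runs an ordered list of tasks one after another.
; On BeginPlay it starts the first task in TaskList.
; CompleteTask walks the list, clearing CanComplete on each task until it finds the completed one, then advances ProgressionIndex and starts the next task.
; Completing the last task starts nothing further, as no end-of-puzzle logic is present.
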(event EventBeginPlay
  (Default|OnStart (Utilities|Array|Get(acopy) (Variables|Default|GetTaskList))))

(fn ConstructionScript)

(fn CompleteTask
  (params (CurrentTask :type BP%20Task%20Object%20Reference))
  (for _index (range 0 (- (Utilities|Array|Length (Variables|Default|GetTaskList)) 1))
    (Variables|/Game/Enigmes/BP_Task.BP_Task_C|SetCanComplete (Utilities|Array|Get(acopy) (Variables|Default|GetTaskList) _index) false)
    (if (== (Utilities|Array|Get(acopy) (Variables|Default|GetTaskList) _index) CurrentTask)
      (bind _output_get (Variables|Default|SetProgressionIndex _index))
      (bind _result (Math|Integer|IncrementInt _output_get)
        (:%20%20
          (if (< _result (Utilities|Array|Length (Variables|Default|GetTaskList)))
            (Default|OnStart (Utilities|Array|Get(acopy) (Variables|Default|GetTaskList) (Variables|Default|GetProgressionIndex)))
            (return)))))))