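; BP_Trigger_Carpet is a carpet trigger that fires configured game events when its state is toggled.
; ToggleState loops over EventsToTrigger and passes the EventEnum of each entry whose EnterOrExit flag is false to CallEventTrigger.
; GetState always returns false, so the trigger tracks no state of its own.
; BeginPlay, overlap and Tick are disabled stubs, and the construction script only calls its parent.
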(event EventBeginPlay
  (|CallParentFunction) ; This node is disabled and will not be called.\nDrag off pins to build functionality.
)

(event Collision|EventActorBeginOverlap
  (params (OtherActor :type Actor%20Object%20Reference)))

(event EventTick
  (params (DeltaSeconds :type Float%20%28single-precision%29)))

(event EventToggleState
  (bind _array_element (Utilities|Array|ForEachLoopwithBreak (Variables|Default|GetEventsToTrigger))
    (:LoopBody
      (if (not (.EnterOrExit (Utilities|Struct|BreakEventType _array_element)))
        (CallFunction|CallEventTrigger (.EventEnum (Utilities|Struct|BreakEventType _array_element)))))))

(fn ConstructionScript
  (|CallParentFunction))

(fn GetState
  (return false))