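; BP_TriggerInteract is a trigger zone variant that fires configured game events on interaction rather than on overlap.
; ToggleState prints a debug string, then loops over EventsToTrigger and passes each EventEnum whose EnterOrExit flag is false to CallEventTrigger.
; Begin and end overlap on TriggerZone only print "Do nothing", and GetState always returns false, so no toggle state is tracked.
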(event OnComponentBeginOverlap(TriggerZone)
  (params (OverlappedComponent :type Primitive%20Component%20Object%20Reference) (OtherActor :type Actor%20Object%20Reference) (OtherComp :type Primitive%20Component%20Object%20Reference) (OtherBodyIndex :type Integer) (bFromSweep :type Boolean) (SweepResult :type Hit%20Result%20Structure%20%28by%20ref%29))
  (Development|PrintString "Do nothing"))

(event OnComponentEndOverlap(TriggerZone)
  (params (OverlappedComponent :type Primitive%20Component%20Object%20Reference) (OtherActor :type Actor%20Object%20Reference) (OtherComp :type Primitive%20Component%20Object%20Reference) (OtherBodyIndex :type Integer))
  (Development|PrintString "Do nothing"))

(event EventBeginPlay
  (|CallParentFunction) ; This node is disabled and will not be called.\nDrag off pins to build functionality.
)

(event Collision|EventActorBeginOverlap
  (params (OtherActor :type Actor%20Object%20Reference)))

(event EventTick
  (params (DeltaSeconds :type Float%20%28single-precision%29)))

(event EventToggleState
  (Development|PrintString "Interact ")
  (bind _array_element (Utilities|Array|ForEachLoopwithBreak (Variables|Default|GetEventsToTrigger))
    (:LoopBody
      (if (not (.EnterOrExit (Utilities|Struct|BreakEventType _array_element)))
        (CallFunction|CallEventTrigger (.EventEnum (Utilities|Struct|BreakEventType _array_element)))))))

(fn ConstructionScript
  (|CallParentFunction))

(fn GetState
  (return false))