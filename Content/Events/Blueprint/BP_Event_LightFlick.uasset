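; Triggerable event Blueprint that makes a spotlight flicker for a set duration.
; TriggerEvent raises a Flick flag, and Tick then drives intensity with a time-based sine, randomized each frame and scaled by the intensity cached at BeginPlay.
; A Delay inside Tick clears the flag after FlickDuration, then either switches the light off or restores its original intensity, depending on LightOffAfterFlick.
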(event EventBeginPlay
  (Variables|Default|SetlightIntensity (Variables|/Script/Engine.LightComponentBase|GetIntensity (Variables|Default|GetSpotLight))))

(event EventTick
  (params (DeltaSeconds :type Float%20%28single-precision%29))
  (bind _flickpower (Variables|Default|GetFlickPower))
  (if (Variables|Default|GetbFlick)
    (Rendering|Components|Light|SetIntensity (Variables|Default|GetSpotLight) (* (Math|Trig|Sin(Radians) (* (Utilities|Time|GetTimeSeconds) _flickpower (Math|Random|RandomFloatinRange 0.0 _flickpower))) (Variables|Default|GetlightIntensity)))
    (Utilities|FlowControl|Delay (Variables|Default|GetFlickDuration))
    (Variables|Default|SetbFlick false)
    (if (Variables|Default|GetLightOffAfterFlick)
      (Rendering|Components|Light|SetIntensity (Variables|Default|GetSpotLight) 0.0)
      (else
        (Rendering|Components|Light|SetIntensity (Variables|Default|GetSpotLight) (Variables|Default|GetlightIntensity))))))

(event EventTriggerEvent
  (Variables|Default|SetbFlick true))

(fn ConstructionScript
  (|CallParentFunction))