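; BP_Event_Sound is an event Blueprint that plays its Audio component when triggered, with a cooldown between replays.
; TriggerEvent plays the sound from the start only when ActualDelay has run out, then resets that timer to TimeAfterReplay.
; Tick continuously counts ActualDelay down by delta time, and the construction script only calls the parent's version.
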(event EventBeginPlay)

(event EventTick
  (params (DeltaSeconds :type Float%20%28single-precision%29))
  (Variables|Default|SetActualDelay (- (Variables|Default|GetActualDelay) DeltaSeconds)))

(event EventTriggerEvent
  (if (<= (Variables|Default|GetActualDelay) 0.0)
    (Audio|Components|Audio|Play (Variables|Default|GetAudio) 0.0)
    (Variables|Default|SetActualDelay (Variables|Default|GetTimeAfterReplay))))

(fn ConstructionScript
  (|CallParentFunction))