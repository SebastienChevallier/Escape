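; Hallucination event actor that gradually distorts the screen through the level's post-process volume once triggered.
; BeginPlay creates a dynamic instance of the volume's first post-process material, and TriggerEvent swaps it in and enables blending.
; Tick ramps a clamped power value over about ten seconds, raising post-process intensity and scaling a time-based sine that drives the material's Speed parameter, which is also debug-printed.
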(event EventBeginPlay
  (bind _returnvalue (Actor|GetActorOfClass "/Script/Engine.PostProcessVolume"))
  (Variables|Default|SetPostProcessVolume _returnvalue)
  (bind _asmaterial (Utilities|Casting|CastToMaterial (.Object (Utilities|Struct|BreakWeightedBlendable (Utilities|Array|Get(acopy) (Utilities|Struct|BreakWeightedBlendables (Utilities|Struct|BreakPostProcessSettings (Variables|/Script/Engine.PostProcessVolume|GetSettings (Variables|Default|GetPostProcessVolume)))))))))
  (bind _returnvalue_2 (Rendering|Material|CreateDynamicMaterialInstance _asmaterial "None" "None" :!class /Script/Engine.KismetMaterialLibrary))
  (Variables|Default|SetmaterialInstance _returnvalue_2))

(event EventTick
  (params (DeltaSeconds :type Float%20%28single-precision%29))
  (if (Variables|Default|GetcanLerp)
    (Variables|Default|SetPowerMultiply (Math|Float|Clamp(Float) (+ (* DeltaSeconds 0.1) (Variables|Default|GetPowerMultiply))))
    (Development|PrintString (Utilities|String|ToString(Float) (Math|Float|Lerp 0.0 2.0 (* (* (Math|Trig|Sin(Radians) (Actor|GetGameTimeSinceCreation)) (Math|Float|Clamp(Float) (+ (* DeltaSeconds 0.1) (Variables|Default|GetPowerMultiply)))) 1.0))) true true "(R=1.000000,G=0.000000,B=0.009249,A=1.000000)" 0.0)
    (Utilities|Struct|SetmembersinPostProcessSettings (Variables|/Script/Engine.PostProcessVolume|GetSettings (Variables|Default|GetPostProcessVolume)) (Math|Float|Lerp 0.0 1.0 (Math|Float|Clamp(Float) (+ (* DeltaSeconds 0.1) (Variables|Default|GetPowerMultiply)))))
    (Rendering|Material|SetScalarParameterValue (Variables|Default|GetmaterialInstance) "Speed" (Math|Float|Lerp 0.0 2.0 (* (* (Math|Trig|Sin(Radians) (Actor|GetGameTimeSinceCreation)) (Math|Float|Clamp(Float) (+ (* DeltaSeconds 0.1) (Variables|Default|GetPowerMultiply)))) 1.0)) :!class /Script/Engine.MaterialInstanceDynamic)))

(event EventTriggerEvent
  (Variables|Default|SetcanLerp true)
  (Utilities|Struct|SetmembersinWeightedBlendable (Utilities|Array|Get(acopy) (Utilities|Struct|BreakWeightedBlendables (Utilities|Struct|BreakPostProcessSettings (Variables|/Script/Engine.PostProcessVolume|GetSettings (Variables|Default|GetPostProcessVolume))))) (Variables|Default|GetmaterialInstance)))

(fn ConstructionScript
  (|CallParentFunction))