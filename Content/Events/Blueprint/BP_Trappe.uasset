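; BP_Trappe is an event-driven hatch actor that opens by playing an actor sequence once it has been unlocked.
; TriggerEvent sets CanBeOpened, and ToggleState plays the sequence only when that flag is true.
; Both events print debug strings, GetState always returns false, and nothing here reverses the sequence or clears the flag.
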(event EventBeginPlay)

(event Collision|EventActorBeginOverlap
  (params (OtherActor :type Actor%20Object%20Reference)))

(event EventTick
  (params (DeltaSeconds :type Float%20%28single-precision%29)))

(event EventTriggerEvent
  (Development|PrintString "Trappe")
  (Variables|Default|SetcanBeOpened true))

(event EventToggleState
  (Development|PrintString "open trappe")
  (if (Variables|Default|GetcanBeOpened)
    (Class|ActorSequenceComponent|PlaySequence (Variables|Default|GetActorSequence))))

(fn ConstructionScript
  (|CallParentFunction))

(fn GetState
  (return false))